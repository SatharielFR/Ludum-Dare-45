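; Parent enemy Blueprint, by its name, that drifts in a straight line at a random velocity.
; BeginPlay rolls non-negative X and Z components up to NbMaxSpeed into VecDirection, leaving Y at zero.
; Tick adds that vector to the actor location without sweep or delta-time scaling, so speed depends on frame rate.
; The construction script applies FScale to the Enemy component's X and Y scale.
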(event EventBeginPlay
  (bind _nbmaxspeed (Variables|Default|GetnbMaxSpeed))
  (bind _returnvalue (Math|Conversions|ToFloat(Integer) _nbmaxspeed))
  ;[1 1 1] Set velocity
  (Variables|Default|SetvecDirection (Math|Vector|MakeVector (Math|Random|RandomFloatinRange 0.0 _returnvalue) 0.0 (Math|Random|RandomFloatinRange 0.0 _returnvalue))))

(event Collision|EventActorBeginOverlap
  (params (OtherActor :type Actor%20Object%20Reference)))

(event EventTick
  (params (DeltaSeconds :type Float%20%28single-precision%29))
  (Transformation|SetActorLocation (+ (Transformation|GetActorLocation) (Variables|Default|GetvecDirection)) false false))

(fn ConstructionScript
  (bind _enemy (Variables|Default|Getenemy))
  (bind _fscale (Variables|Default|GetfScale))
  (Rendering|Components|TextRender|SetXScale _enemy _fscale)
  (Rendering|Components|TextRender|SetYScale _enemy _fscale))