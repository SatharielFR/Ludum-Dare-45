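; Enemy spawner Blueprint that creates a short burst of BpParentEnnemy actors around the player pawn after play begins.
; Each Tick spawns one enemy at the player's location plus a random unit vector, passes it scale and max-speed values, and increments the count.
; Once the count exceeds the maximum set at BeginPlay, it is pinned to a higher constant, so spawning stops.
; An inner comparison of two constants always passes.
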(event EventBeginPlay
  (Variables|Default|SetnbEnnemyPresent 0)
  (Variables|Default|SetnbEnemyMax 3)
  (Variables|Default|SetfScale 1.0)
  (Variables|Default|SetnbMaxSpeed 1))

(event Collision|EventActorBeginOverlap
  (params (OtherActor :type Actor%20Object%20Reference)))

(event EventTick
  (params (DeltaSeconds :type Float%20%28single-precision%29))
  (if (<= (Variables|Default|GetnbEnnemyPresent) (Variables|Default|GetnbEnemyMax))
    (if (>= 0.0 0.0)
      (bind _returnvalue (Game|SpawnActorfromClass "/Game/Blueprint/Ennemy/bpParentEnnemy.bpParentEnnemy_C" (Math|Conversions|ToTransform(Vector) (+ (Math|Random|RandomUnitVector) (Transformation|GetActorLocation (Game|Player|GetPlayerPawn 0)))) "Undefined" 0 0))
      (bind _asbp_parent_ennemy (Utilities|Casting|CastTobpParentEnnemy _returnvalue))
      (Variables|/Game/Blueprint/Ennemy/bpParentEnnemy.bpParentEnnemy_C|SetfScale _asbp_parent_ennemy (Variables|Default|GetfScale))
      (Variables|/Game/Blueprint/Ennemy/bpParentEnnemy.bpParentEnnemy_C|SetnbMaxSpeed _asbp_parent_ennemy (Variables|Default|GetnbMaxSpeed))
      ;[1 1 1] Increment NbEnemy Variable
      (Variables|Default|SetnbEnnemyPresent (+ (Variables|Default|GetnbEnnemyPresent) 1))
      (else
        (Variables|Default|SetnbEnnemyPresent 10 :!label _label)))
    (else
      (goto _label))))

(fn ConstructionScript)