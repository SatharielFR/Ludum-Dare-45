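; Player character for a Paper2D game, moving on the X/Z plane from axis input and turning to face the mouse cursor.
; Each tick derives the Sprite's pitch from the cursor's offset to viewport center using arccosine, mirrored by the Y sign.
; Tick also reapplies a fixed walk sprite and drains NbRage about once per second through a Delay.
; SetMyFlipbook, a movement-based animation selector, is never run.
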(event Custom|Tick%202
  (if (> (Variables|Default|GetnbRage) 0.0)
    (Utilities|FlowControl|Delay 1.0)
    (Variables|Default|SetnbRage (- (Variables|Default|GetnbRage) 2.0))))

(event Custom|Tick1
  (Rendering|Components|Sprite|SetSprite (Variables|Default|GetPaperSprite) "/Game/Model3D/Animation_walk_Sprite_0.Animation_walk_Sprite_0"))

(event Custom|Tick%203
  (bind _returnvalue (Game|GetPlayerController 0))
  (bind (_sizex _sizey) (HUD|GetViewportSize _returnvalue))
  (bind (_locationx _locationy) (Game|Player|GetMousePosition _returnvalue))
  (bind _returnvalue_2 (/ _sizey 2))
  (bind _returnvalue_3 (Math|Vector2D|MakeVector2D _locationx _locationy))
  (bind _returnvalue_4 (/ _sizex 2))
  (bind _returnvalue_5 (Math|Conversions|ToFloat(Integer) _returnvalue_2))
  (bind _returnvalue_6 (Math|Conversions|ToFloat(Integer) _returnvalue_4))
  (bind _returnvalue_7 (Math|Vector2D|MakeVector2D _returnvalue_6 _returnvalue_5))
  (bind _returnvalue_8 (- _returnvalue_3 _returnvalue_7))
  (bind _returnvalue_9 (Math|Vector|Distance2D(Vector) _returnvalue_3 _returnvalue_7))
  (bind _returnvalue_10 (/ (.x _returnvalue_8) _returnvalue_9))
  (bind _returnvalue_11 (Class|KismetMathLibrary|DegAcos _returnvalue_10))
  (if (> (/ (.y _returnvalue_8) _returnvalue_9) 0.0)
    (Transformation|SetRelativeRotation (Variables|Default|GetSprite) (Math|Rotator|MakeRotator 0.0 (+ (* _returnvalue_11 -1.0) 9e+01) 0.0) false false)
    (else
      (Transformation|SetRelativeRotation (Variables|Default|GetSprite) (Math|Rotator|MakeRotator 0.0 (+ _returnvalue_11 9e+01) 0.0) false false))))

(event EventBeginPlay
  (Variables|/Script/Engine.PlayerController|SetbShowMouseCursor (Game|GetPlayerController 0) true))

(event EventTick
  (params (DeltaSeconds :type Float%20%28single-precision%29))
  (CallFunction|Tick1)
  (CallFunction|Tick3)
  (CallFunction|Tick2))

(event Input|AxisEvents|InputAxisUpOrDown
  (params (AxisValue :type Float%20%28single-precision%29))
  (Pawn|Input|AddMovementInput "0, 0,1.000000" AxisValue false))

(event Input|AxisEvents|InputAxisLeftOrRight
  (params (AxisValue :type Float%20%28single-precision%29))
  (Pawn|Input|AddMovementInput "1.000000, 0, 0" AxisValue false))

(fn ConstructionScript)

(fn SetMyFlipbook
  (if (or (!= (Input|AxisValues|GetLeftOrRight) 0.0) (!= (Input|AxisValues|GetUpOrDown) 0.0))
    (Variables|Default|SetLastMoveDirection (select (> (Input|AxisValues|GetUpOrDown) 0.0) "NewEnumerator0" (select (< (Input|AxisValues|GetUpOrDown) 0.0) "NewEnumerator1" (select (> (Input|AxisValues|GetLeftOrRight) 0.0) "NewEnumerator3" "NewEnumerator2")))))
  (Sprite|SetFlipbook (Variables|Default|GetSprite) (select (> (Math|Vector|VectorLength (Transformation|GetVelocity)) 0.0) (Utilities|Select :Index (Variables|Default|GetLastMoveDirection) :NewEnumerator0 "/Game/Model3D/MoveDown.MoveDown" :NewEnumerator1 "/Game/Model3D/MoveDown.MoveDown" :NewEnumerator2 "/Game/Model3D/MoveDown.MoveDown" :NewEnumerator3 "/Game/Model3D/MoveDown.MoveDown") (Utilities|Select :Index (Variables|Default|GetLastMoveDirection) :NewEnumerator0 "/Game/Model3D/IdleDown.IdleDown" :NewEnumerator1 "/Game/Model3D/IdleDown.IdleDown" :NewEnumerator2 "/Game/Model3D/IdleDown.IdleDown" :NewEnumerator3 "/Game/Model3D/IdleDown.IdleDown"))))